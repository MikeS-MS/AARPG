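; BP_SkillInventory is a player skill component that looks up the level of the owning character's abilities.
; On BeginPlay it casts its owner to BP_RPGPlayerCharacter and caches it as OwningPlayer.
; GetSkillValue returns a level from the AbilityLevels map only when the owner's AbilityInventory contains that ability, otherwise not found and zero.
; AddPointToAbility is an empty stub with disconnected leftover logic for removing an unlocked ability.
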(event EventBeginPlay
  (bind _asbp_rpgplayer_character (Utilities|Casting|CastToBP_RPGPlayerCharacter (Components|GetOwner)))
  (Variables|Instances|SetOwningPlayer _asbp_rpgplayer_character))

(event EventTick
  (params (DeltaSeconds :type Float%20%28single-precision%29)))

(fn AddPointtoAbility
  (params (Ability :type S%20Ability%20Structure)))

(fn GetSkillValue
  (params (Ability :type S%20Ability%20Structure))
  (bind _abilitylevels (Variables|Default|GetAbilityLevels))
  (bind (_value _returnvalue) (Utilities|Map|Find _abilitylevels Ability))
  (if (Default|AbilityExists (Variables|/Game/Blueprints/Characters/Player/BP_RPGPlayerCharacter.BP_RPGPlayerCharacter_C|GetAbilityInventory (Variables|Instances|GetOwningPlayer)) Ability)
    (return _returnvalue _value)
    (else
      (return false 0))))