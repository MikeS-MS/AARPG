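; Player skill component that holds a Skills array and serves as a lookup for the value of a named skill at its current level.
; GetSkillValue matches the name case-insensitively, skips entries with a negative level, and indexes that skill's Values array by its level.
; It returns an empty string when nothing matches, and the event graph has no active logic.
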(event EventBeginPlay)

(event EventTick
  (params (DeltaSeconds :type Float%20%28single-precision%29)))

(fn GetSkillValue
  (params (SkillName :type String))
  (for _array_element (Variables|Default|GetSkills)
    (if (and (> (.skilllevel _array_element) -1) (Utilities|Enum|Equal(Enum) (Utilities|String|ToLower (.skillname _array_element)) (Utilities|String|ToLower SkillName)))
      (return (Utilities|Array|Get(acopy) (.values _array_element) (.skilllevel _array_element)))))
  (return ""))