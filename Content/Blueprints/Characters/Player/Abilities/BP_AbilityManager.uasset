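; BP_AbilityManager computes the damage list and extra stats of a character's ability from base and per-level tables.
; GetStats reads the skill level from the character's SkillInventory, returning unscaled base stats if no per-level data or skill is found.
; Damage entries, paired by index, scale with level and the player's damage type multipliers; entries failing match or lookup are dropped.
; Extra stats scale linearly, with Timer decreasing per level.
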(fn GetStats
  (params (Ability :type S%20Ability%20Structure) (Character :type BP%20RPG%20Player%20Character%20Object%20Reference))
  (bind _abilitystatsbase (Variables|Default|GetAbilityStatsBase))
  (bind _abilitystatsperlevel (Variables|Default|GetAbilityStatsPerLevel))
  (bind _skillinventory (Variables|/Game/Blueprints/Characters/Player/BP_RPGPlayerCharacter.BP_RPGPlayerCharacter_C|GetSkillInventory Character))
  (bind (_value _returnvalue) (Utilities|Map|Find _abilitystatsperlevel Ability))
  (bind (_value_2 _returnvalue_2) (Utilities|Map|Find _abilitystatsbase Ability))
  (bind (_found _level) (Default|GetSkillValue _skillinventory Ability))
  (if _returnvalue_2
    (if (and _returnvalue _found)
      (return true (Utilities|Struct|MakeS_AbilityDamagesAndStats (CallFunction|AccumulateDamageLists (.damage _value_2) (.damage _value) _level Character) (CallFunction|AccumulateStats (.extrastats _value_2) (.extrastats _value) _level)))
      (else
        (return true (Utilities|Struct|MakeS_AbilityDamagesAndStats (.damage _value_2) (.extrastats _value_2)))))
    (else
      (return false ""))))

(fn AccumulateDamageLists
  (params (Base :type Array%20of%20S%20Damage%20Structures) (PerLevel :type Array%20of%20S%20Damage%20Structures) (Level :type Integer) (Player :type BP%20RPG%20Player%20Character%20Object%20Reference))
  (bind _temp (LocalVariables|GetTemp))
  (bind _statsinventory (Variables|/Game/Blueprints/Characters/BP_BaseCharacter.BP_BaseCharacter_C|GetStatsInventory Player))
  (bind _statsmanager (Variables|/Game/Blueprints/Characters/Stats/BP_StatsInventory.BP_StatsInventory_C|GetStatsManager _statsinventory))
  (bind _stats (Variables|/Game/Blueprints/Characters/Stats/BP_StatsInventory.BP_StatsInventory_C|GetStats _statsinventory))
  (for (_array_element _array_index) Base
    (if (Math|Boolean|ANDBoolean (Utilities|Enum|Equal(Enum) (.damagetype _array_element) (.damagetype (Utilities|Array|Get(acopy) PerLevel _array_index))) (Math|Boolean|Equal(Boolean) (.statuseffect _array_element) (.statuseffect (Utilities|Array|Get(acopy) PerLevel _array_index))) (.Found (Default|GetDamagesEntry _statsmanager (.damagetype _array_element))) (.Found (Default|GetCharacterDamageTypeValue _statsmanager (.damagetype (.damagetype _stats)) (.DamageTypeMultipliers (Default|GetDamagesEntry _statsmanager (.damagetype _array_element))))))
      (Utilities|Array|Add _temp (Utilities|Struct|MakeS_Damage (.damagetype (Utilities|Array|Get(acopy) PerLevel _array_index)) (* (* (* (.Value (Default|GetDamagesEntry _statsmanager (.damagetype _array_element))) (.Value (Default|GetCharacterDamageTypeValue _statsmanager (.damagetype (.damagetype _stats)) (.DamageTypeMultipliers (Default|GetDamagesEntry _statsmanager (.damagetype _array_element)))))) (.damage (.damagetype _stats))) (+ (.value _array_element) (* Level (.value (Utilities|Array|Get(acopy) PerLevel _array_index))))) (.statuseffect (Utilities|Array|Get(acopy) PerLevel _array_index))))))
  (return _temp))

(fn AccumulateStats
  (params (Base :type S%20Ability%20Extra%20Stats%20Structure) (PerLevel :type S%20Ability%20Extra%20Stats%20Structure) (Level :type Integer))
  (bind (_speed _xrange _yrange _force _timer _stay _projectiles) (Utilities|Struct|BreakS_AbilityExtraStats Base))
  (bind (_speed_2 _xrange_2 _yrange_2 _force_2 _timer_2 _stay_2 _projectiles_2) (Utilities|Struct|BreakS_AbilityExtraStats PerLevel))
  (return (Utilities|Struct|MakeS_AbilityExtraStats (+ _speed (* Level _speed_2)) (+ _xrange (* Level _xrange_2)) (+ _yrange (* Level _yrange_2)) (+ _force (* Level _force_2)) (- _timer (* Level _timer_2)) (+ _stay (* Level _stay_2)) (+ _projectiles (* Level _projectiles_2)))))