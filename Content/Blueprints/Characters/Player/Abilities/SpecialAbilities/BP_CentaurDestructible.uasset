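; BP_CentaurDestructible is a breakable actor, filed under player special abilities, that shatters on demand and then cleans itself up.
; Fracture applies full radius damage at the Destructible component's own location, using configurable radius and impulse force, with a flag so it fires only once.
; It then starts a timer by function name that destroys the actor after TimeToStay.
; The event graph and construction script are empty, so breaking relies on Fracture being called.
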(event EventBeginPlay)

(event Collision|EventActorBeginOverlap
  (params (OtherActor :type Actor%20Object%20Reference)))

(event EventTick
  (params (DeltaSeconds :type Float%20%28single-precision%29)))

(fn ConstructionScript)

(fn Fracture
  (bind _destructible (Variables|Default|GetDestructible))
  (if (not (Variables|Default|GetDestroyed))
    (Class|DestructibleComponent|ApplyRadiusDamage _destructible 1.0 (Transformation|GetWorldLocation _destructible) (Variables|Default|GetRadius) (Variables|Default|GetForce) true)
    (Utilities|Time|SetTimerbyFunctionName self "DestroyDestructibleActor" (Variables|Default|GetTimeToStay))
    (Variables|Default|SetDestroyed true)))

(fn DestroyDestructibleActor
  (Actor|DestroyActor))