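; Segment of a wind current that carries an RPG player who has a specific ability along a cylinder to its end zone.
; Entering the cylinder stops casting, sets flying and adds a status effect.
; Tick then sweeps the player toward the end zone at the ability's speed.
; Exiting, blocking hits or reaching the end restore falling and clear the effect, with the end zone adding a launch impulse along the cylinder's up axis.
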(event OnComponentBeginOverlap(Cylinder)
  (params (OverlappedComponent :type Primitive%20Component%20Object%20Reference) (OtherActor :type Actor%20Object%20Reference) (OtherComp :type Primitive%20Component%20Object%20Reference) (OtherBodyIndex :type Integer) (bFromSweep :type Boolean) (SweepResult :type Hit%20Result%20Structure%20%28by%20ref%29))
  (bind _s_ability (Utilities|Struct|MakeS_Ability "NewEnumerator2" "NewEnumerator1"))
  (bind _asbp_rpgplayer_character (Utilities|Casting|CastToBP_RPGPlayerCharacter OtherActor))
  (if (== (Variables|/Script/Engine.Character|GetCapsuleComponent _asbp_rpgplayer_character) OtherComp)
    (if (.Found (Default|GetAbilityStatus (Variables|/Game/Blueprints/Characters/Player/BP_RPGPlayerCharacter.BP_RPGPlayerCharacter_C|GetAbilityInventory _asbp_rpgplayer_character) _s_ability))
      (Default|WindUTimerClear (Variables|/Game/Blueprints/Characters/Player/BP_RPGPlayerCharacter.BP_RPGPlayerCharacter_C|GetAbilityInventory _asbp_rpgplayer_character))
      (Default|SetCasting (Variables|/Game/Blueprints/Characters/Player/BP_RPGPlayerCharacter.BP_RPGPlayerCharacter_C|GetAbilityInventory _asbp_rpgplayer_character) _s_ability false)
      (bind _output_get (Variables|Default|SetPlayer _asbp_rpgplayer_character))
      (Pawn|Components|CharacterMovement|SetMovementMode (Variables|/Script/Engine.Character|GetCharacterMovement _output_get) "MOVE_Flying" 0)
      (Components|Movement|StopMovementImmediately (Variables|/Script/Engine.Character|GetCharacterMovement _output_get))
      (Default|AddStatusEffect (Variables|/Game/Blueprints/Characters/BP_BaseCharacter.BP_BaseCharacter_C|GetStatusEffectInventory _output_get) "NewEnumerator5" _output_get (Utilities|Array|MakeArray) false))))

(event OnComponentEndOverlap(Cylinder)
  (params (OverlappedComponent :type Primitive%20Component%20Object%20Reference) (OtherActor :type Actor%20Object%20Reference) (OtherComp :type Primitive%20Component%20Object%20Reference) (OtherBodyIndex :type Integer))
  (bind _asbp_rpgplayer_character (Utilities|Casting|CastToBP_RPGPlayerCharacter OtherActor))
  (if (== (Variables|/Script/Engine.Character|GetCapsuleComponent _asbp_rpgplayer_character) OtherComp)
    (CallFunction|Detach)))

(event OnComponentBeginOverlap(EndZone)
  (params (OverlappedComponent :type Primitive%20Component%20Object%20Reference) (OtherActor :type Actor%20Object%20Reference) (OtherComp :type Primitive%20Component%20Object%20Reference) (OtherBodyIndex :type Integer) (bFromSweep :type Boolean) (SweepResult :type Hit%20Result%20Structure%20%28by%20ref%29))
  (bind _asbp_rpgplayer_character (Utilities|Casting|CastToBP_RPGPlayerCharacter OtherActor))
  (if (== (Variables|/Script/Engine.Character|GetCapsuleComponent _asbp_rpgplayer_character) OtherComp)
    (CallFunction|Detach)
    (if (.Found (Default|GetAbilityStatus (Variables|/Game/Blueprints/Characters/Player/BP_RPGPlayerCharacter.BP_RPGPlayerCharacter_C|GetAbilityInventory _asbp_rpgplayer_character) (Utilities|Struct|MakeS_Ability "NewEnumerator2" "NewEnumerator1")))
      (Physics|AddImpulse (Variables|/Script/Engine.Character|GetCharacterMovement _asbp_rpgplayer_character) (* (Math|Vector|GetUpVector (Variables|Default|GetCylinder)) (.speed (.extrastats (.damage (.CD (Default|GetAbilityStatus (Variables|/Game/Blueprints/Characters/Player/BP_RPGPlayerCharacter.BP_RPGPlayerCharacter_C|GetAbilityInventory _asbp_rpgplayer_character) (Utilities|Struct|MakeS_Ability "NewEnumerator2" "NewEnumerator1"))))))) true))))

(event EventBeginPlay)

(event Collision|EventActorBeginOverlap
  (params (OtherActor :type Actor%20Object%20Reference)))

(event EventTick
  (params (DeltaSeconds :type Float%20%28single-precision%29))
  (CallFunction|MovePlayer DeltaSeconds))

(fn ConstructionScript)

(fn MovePlayer
  (params (DeltaTime :type Float%20%28single-precision%29))
  (bind _player (Variables|Default|GetPlayer))
  (bind _abilityinventory (Variables|/Game/Blueprints/Characters/Player/BP_RPGPlayerCharacter.BP_RPGPlayerCharacter_C|GetAbilityInventory _player))
  (bind (_found _cd) (Default|GetAbilityStatus _abilityinventory (Utilities|Struct|MakeS_Ability "NewEnumerator2" "NewEnumerator1")))
  (Utilities|IsValid _player
    (:Is%20Valid
      (if _found
        (bind (_sweephitresult _returnvalue) (Transformation|SetActorLocation _player (Math|Interpolation|VInterptoConstant (Transformation|GetActorLocation _player) (Transformation|GetWorldLocation (Variables|Default|GetEnd%20Zone)) DeltaTime (.speed (.extrastats (.damage _cd)))) true true))
        (if (and (.bblockinghit _sweephitresult) _returnvalue)
          (CallFunction|Detach :!label _label))
        (else
          (goto _label))))))

(fn Detach
  (Utilities|IsValid (Variables|Default|GetPlayer)
    (:Is%20Valid
      (if (.Found (Default|GetAbilityStatus (Variables|/Game/Blueprints/Characters/Player/BP_RPGPlayerCharacter.BP_RPGPlayerCharacter_C|GetAbilityInventory (Variables|Default|GetPlayer)) (Utilities|Struct|MakeS_Ability "NewEnumerator2" "NewEnumerator1")))
        (Default|WindUReset (Variables|/Game/Blueprints/Characters/Player/BP_RPGPlayerCharacter.BP_RPGPlayerCharacter_C|GetAbilityInventory (Variables|Default|GetPlayer))))
      (Pawn|Components|CharacterMovement|SetMovementMode (Variables|/Script/Engine.Character|GetCharacterMovement (Variables|Default|GetPlayer)) "MOVE_Falling" 0)
      (bind (_exists _effect) (Default|EffectExists (Variables|/Game/Blueprints/Characters/BP_BaseCharacter.BP_BaseCharacter_C|GetStatusEffectInventory (Variables|Default|GetPlayer)) "NewEnumerator5"))
      (if _exists
        (Default|RemoveStatusEffect (Variables|/Game/Blueprints/Characters/BP_BaseCharacter.BP_BaseCharacter_C|GetStatusEffectInventory (Variables|Default|GetPlayer)) _effect)))
    (:Is%20Not%20Valid
      _))
  (Variables|Default|SetPlayer 0))