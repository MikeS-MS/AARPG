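; Grapple point actor for the player's grappling ability, pulling an attached player toward a target point.
; Attach stores player, speed and point and spawns a BP_Vine if none is valid.
; Tick moves the player by constant-speed interpolation with a swept move, detaching on a blocking hit or on reaching DetachZone.
; Detach restores walking, clears the ability's casting state and a status effect, then tells the vine to move towards center.
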(event OnComponentBeginOverlap(DetachZone)
  (params (OverlappedComponent :type Primitive%20Component%20Object%20Reference) (OtherActor :type Actor%20Object%20Reference) (OtherComp :type Primitive%20Component%20Object%20Reference) (OtherBodyIndex :type Integer) (bFromSweep :type Boolean) (SweepResult :type Hit%20Result%20Structure%20%28by%20ref%29))
  (bind _asbp_rpgplayer_character (Utilities|Casting|CastToBP_RPGPlayerCharacter OtherActor))
  (Variables|Default|SetInside true)
  (if (== _asbp_rpgplayer_character (Variables|Default|GetPlayer))
    (CallFunction|Detach)))

(event OnComponentEndOverlap(DetachZone)
  (params (OverlappedComponent :type Primitive%20Component%20Object%20Reference) (OtherActor :type Actor%20Object%20Reference) (OtherComp :type Primitive%20Component%20Object%20Reference) (OtherBodyIndex :type Integer))
  (Utilities|Casting|CastToBP_RPGPlayerCharacter OtherActor)
  (Variables|Default|SetInside false))

(event EventBeginPlay)

(event Collision|EventActorBeginOverlap
  (params (OtherActor :type Actor%20Object%20Reference)))

(event EventTick
  (params (DeltaSeconds :type Float%20%28single-precision%29))
  (bind _player (Variables|Default|GetPlayer))
  (Utilities|IsValid _player
    (:Is%20Valid
      (bind _sweephitresult (Transformation|SetActorLocation _player (Math|Interpolation|VInterptoConstant (Transformation|GetActorLocation _player) (Variables|Default|GetPoint) DeltaSeconds (Variables|Default|GetSpeed)) true true))
      (if (.bblockinghit _sweephitresult)
        (CallFunction|Detach)))))

(fn ConstructionScript)

(fn Attach
  (params (Player :type BP%20RPG%20Player%20Character%20Object%20Reference) (Speed :type Float%20%28single-precision%29) (Point :type Vector))
  (Variables|Default|SetPlayer Player)
  (Variables|Default|SetSpeed Speed)
  (Variables|Default|SetPoint Point)
  (Utilities|IsValid (Variables|Instances|GetVine)
    (:Is%20Not%20Valid
      (bind _returnvalue (Game|SpawnActorfromClass "/Game/Blueprints/Characters/Player/Abilities/VisualFX/BP_Vine.BP_Vine_C" (Math|Transform|MakeTransform "0, 0, 0" "0, 0, 0" "1,1,1") "Undefined" 0 0))
      (Variables|Instances|SetVine _returnvalue)
      (Default|Setup _returnvalue (Variables|/Game/Blueprints/Characters/Player/BP_RPGPlayerCharacter.BP_RPGPlayerCharacter_C|GetVinePosition (Variables|Default|GetPlayer)) false false Speed Point))))

(fn Detach
  (bind _s_ability (Utilities|Struct|MakeS_Ability "NewEnumerator2" "NewEnumerator0"))
  (bind _vine (Variables|Instances|GetVine))
  (Utilities|IsValid (Variables|Default|GetPlayer)
    (:Is%20Valid
      (Pawn|Components|CharacterMovement|SetMovementMode (Variables|/Script/Engine.Character|GetCharacterMovement (Variables|Default|GetPlayer)) "MOVE_Walking" 0)
      (if (.iscasting (.CD (Default|GetAbilityStatus (Variables|/Game/Blueprints/Characters/Player/BP_RPGPlayerCharacter.BP_RPGPlayerCharacter_C|GetAbilityInventory (Variables|Default|GetPlayer)) _s_ability)))
        (Default|SetCasting (Variables|/Game/Blueprints/Characters/Player/BP_RPGPlayerCharacter.BP_RPGPlayerCharacter_C|GetAbilityInventory (Variables|Default|GetPlayer)) _s_ability false))
      (bind (_exists _effect) (Default|EffectExists (Variables|/Game/Blueprints/Characters/BP_BaseCharacter.BP_BaseCharacter_C|GetStatusEffectInventory (Variables|Default|GetPlayer)) "NewEnumerator5"))
      (if _exists
        (Default|RemoveStatusEffect (Variables|/Game/Blueprints/Characters/BP_BaseCharacter.BP_BaseCharacter_C|GetStatusEffectInventory (Variables|Default|GetPlayer)) _effect))
      (Variables|Default|SetPlayer 0)
      (Utilities|IsValid _vine
        (:Is%20Valid
          (Default|SetMoveTowardsCenter _vine))))))