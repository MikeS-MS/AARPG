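; BP_MovingLocation is a player special-ability helper actor that follows the player's aim while the ability is casting.
; Attach stores the player, takes speed from the ability's stats and fixes range as the camera-to-actor distance.
; Each tick it moves at constant speed toward the eye-trace hit or max-range point, clearing the player when casting ends.
; Swept moves ignore player characters and offset along other surfaces' hit normals.
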(event EventBeginPlay)

(event Collision|EventActorBeginOverlap
  (params (OtherActor :type Actor%20Object%20Reference)))

(event EventTick
  (params (DeltaSeconds :type Float%20%28single-precision%29))
  (CallFunction|MoveTowardsLocation DeltaSeconds))

(fn ConstructionScript)

(fn MoveTowardsLocation
  (params (DeltaTime :type Float%20%28single-precision%29))
  (bind _returnvalue (Transformation|GetActorLocation))
  (bind _speed (Variables|Default|GetSpeed))
  (bind _range (Variables|Default|GetRange))
  (Utilities|IsValid (Variables|Instances|GetPlayer)
    (:Is%20Valid
      (if (.Found (Default|GetAbilityStatus (Variables|/Game/Blueprints/Characters/Player/BP_RPGPlayerCharacter.BP_RPGPlayerCharacter_C|GetAbilityInventory (Variables|Instances|GetPlayer)) (Utilities|Struct|MakeS_Ability "NewEnumerator2" "NewEnumerator2")))
        (if (.iscasting (.CD (Default|GetAbilityStatus (Variables|/Game/Blueprints/Characters/Player/BP_RPGPlayerCharacter.BP_RPGPlayerCharacter_C|GetAbilityInventory (Variables|Instances|GetPlayer)) (Utilities|Struct|MakeS_Ability "NewEnumerator2" "NewEnumerator2"))))
          (if (.Hit (Default|GetPointatEyes (Variables|Instances|GetPlayer) _range (Utilities|Array|MakeArray (Variables|Instances|GetPlayer) self) true false false false (Default|GetOriginCam (Variables|Instances|GetPlayer))))
            (if (.bblockinghit (.HitResult (Default|GetPointatEyes (Variables|Instances|GetPlayer) _range (Utilities|Array|MakeArray (Variables|Instances|GetPlayer) self) true false false false (Default|GetOriginCam (Variables|Instances|GetPlayer)))))
              (CallFunction|SetLocation (Math|Interpolation|VInterptoConstant _returnvalue (.location (.HitResult (Default|GetPointatEyes (Variables|Instances|GetPlayer) _range (Utilities|Array|MakeArray (Variables|Instances|GetPlayer) self) true false false false (Default|GetOriginCam (Variables|Instances|GetPlayer))))) DeltaTime _speed))
              (else
                (CallFunction|SetLocation (Math|Interpolation|VInterptoConstant _returnvalue (Default|GetEyes (Variables|Instances|GetPlayer) _range) DeltaTime _speed) :!label _label)))
            (else
              (goto _label)))
          (else
            (Variables|Instances|SetPlayer 0 :!label _label_2)))
        (else
          (goto _label_2))))))

(fn Attach
  (params (Player :type BP%20RPG%20Player%20Character%20Object%20Reference))
  (bind _abilityinventory (Variables|/Game/Blueprints/Characters/Player/BP_RPGPlayerCharacter.BP_RPGPlayerCharacter_C|GetAbilityInventory Player))
  (bind (_found _cd) (Default|GetAbilityStatus _abilityinventory (Utilities|Struct|MakeS_Ability "NewEnumerator2" "NewEnumerator2")))
  (Utilities|IsValid Player
    (:Is%20Valid
      (if _found
        (Variables|Instances|SetPlayer Player)
        (Variables|Default|SetSpeed (.speed (.extrastats (.damage _cd))))
        (Variables|Default|SetRange (Math|Vector|Distance(Vector) (Default|GetOriginCam Player) (Transformation|GetActorLocation)))))))

(fn SetLocation
  (params (NewLocation :type Vector))
  (bind _sweephitresult (Transformation|SetActorLocation NewLocation true true))
  (if (.bblockinghit _sweephitresult)
    (Utilities|Casting|CastToBP_RPGPlayerCharacter (.hitactor _sweephitresult)
      (:then
        (Transformation|SetActorLocation NewLocation false true))
      (:CastFailed
        (Transformation|SetActorLocation (+ NewLocation (* (.normal _sweephitresult) (Math|Vector|Distance(Vector) NewLocation (.location _sweephitresult)))) true true)))))