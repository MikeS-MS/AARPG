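; Short-lived visual effect actor that displays a magic circle particle for a player ability's attack.
; On BeginPlay it passes its color and lifetime to the particle component and starts two one-shot timers.
; One fires a fifth of the way through the lifetime to broadcast the attack's OnCircleMaxScale event, and the other destroys the actor when the lifetime ends.
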(event Custom|Event%20Max%20Scale
  (Default|CallOnCircleMaxScale (Variables|Default|GetAttack)))

(event Custom|Destroy
  (Actor|DestroyActor))

(event EventBeginPlay
  (bind _particlelifetimeinseconds (Variables|Default|GetParticleLifetimeInSeconds))
  (bind _magiccircle_p (Variables|Default|GetMagicCircle_P))
  (Effects|Components|ParticleSystem|SetVectorParameter _magiccircle_p "Color" (Math|Conversions|ToVector(LinearColor) (Variables|Default|GetColor)))
  (Effects|Components|ParticleSystem|SetFloatParameter _magiccircle_p "Lifetime" _particlelifetimeinseconds)
  (Utilities|Time|SetTimerbyEvent (delegate Custom|Event%20Max%20Scale) (* _particlelifetimeinseconds 0.2))
  (Utilities|Time|SetTimerbyEvent (delegate Custom|Destroy) _particlelifetimeinseconds))

(fn ConstructionScript)