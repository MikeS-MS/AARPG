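; Visual effect actor for a player ability that draws a vine as a spline mesh anchored to a given actor.
; Setup supplies that actor, target, speed and reverse flag, then Tick extends the vine's end toward the target at constant speed.
; Once extended, it retracts toward the actor if reversed, otherwise holds its end while the start keeps following.
; It destroys itself when both ends meet or the actor becomes invalid.
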(event EventBeginPlay)

(event Collision|EventActorBeginOverlap
  (params (OtherActor :type Actor%20Object%20Reference)))

(event EventTick
  (params (DeltaSeconds :type Float%20%28single-precision%29))
  (Utilities|IsValid self
    (:Is%20Valid
      (if (not (Variables|Default|GetSecondary))
        (CallFunction|FirstMoveVine DeltaSeconds)
        (else
          (CallFunction|SecondaryMoveVine DeltaSeconds))))))

(fn ConstructionScript)

(fn Setup
  (params (Actor :type Actor%20Object%20Reference) (Reverse :type Boolean) (Speed :type Float%20%28single-precision%29) (Location :type Vector))
  (bind _splinemesh (Variables|Default|GetSplineMesh))
  (Utilities|IsValid Actor
    (:Is%20Valid
      (bind _output_get (Variables|Instances|SetActor Actor))
      (Variables|Default|SetReverse Reverse)
      (Variables|Default|SetSpeed Speed)
      (Variables|Default|SetEndLocation Location)
      (SplineMesh|SetStartPosition _splinemesh (Transformation|GetActorLocation _output_get) true)
      (SplineMesh|SetEndPosition _splinemesh (Transformation|GetActorLocation _output_get) true))
    (:Is%20Not%20Valid
      (CallFunction|EndVine))))

(fn FirstMoveVine
  (params (DeltaTime :type Float%20%28single-precision%29))
  (bind _actor (Variables|Instances|GetActor))
  (bind _splinemesh (Variables|Default|GetSplineMesh))
  (bind _endlocation (Variables|Default|GetEndLocation))
  (bind _returnvalue (SplineMesh|GetEndPosition _splinemesh))
  (Utilities|IsValid _actor
    (:Is%20Valid
      (SplineMesh|SetStartPosition _splinemesh (Transformation|GetActorLocation _actor) true)
      (SplineMesh|SetEndPosition _splinemesh (Math|Interpolation|VInterptoConstant _returnvalue _endlocation DeltaTime (* (Variables|Default|GetSpeed) 4.0)) true)
      (if (Math|Vector|Equal(Vector) _returnvalue _endlocation 0.0001)
        (Variables|Default|SetSecondary true)))
    (:Is%20Not%20Valid
      (CallFunction|EndVine))))

(fn SecondaryMoveVine
  (params (DeltaTime :type Float%20%28single-precision%29))
  (bind _actor (Variables|Instances|GetActor))
  (bind _splinemesh (Variables|Default|GetSplineMesh))
  (bind _returnvalue (SplineMesh|GetEndPosition _splinemesh))
  (bind _returnvalue_2 (SplineMesh|GetStartPosition _splinemesh))
  (Utilities|IsValid _actor
    (:Is%20Valid
      (if (Variables|Default|GetReverse)
        (SplineMesh|SetEndPosition _splinemesh (Math|Interpolation|VInterptoConstant _returnvalue _returnvalue_2 DeltaTime (* (Variables|Default|GetSpeed) 4.0)) true))
      (SplineMesh|SetStartPosition _splinemesh (Transformation|GetActorLocation _actor) true)
      (if (Math|Vector|Equal(Vector) _returnvalue _returnvalue_2 0.0001)
        (CallFunction|EndVine)))
    (:Is%20Not%20Valid
      (Actor|DestroyActor))))

(fn EndVine
  (Actor|DestroyActor))

(fn SetReverse
  (Variables|Default|SetReverse true))

(fn GetActor
  (return (Variables|Instances|GetActor)))