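; BP_BaseCharacter is a base character Blueprint that delegates combat stats and status effects to components.
; It recalculates stats on BeginPlay through StatsInventory and forwards Hit calls, with damage, attacker and first-hit argument, to that component.
; Kill only clears all effects in StatusEffectInventory, and IsDead reports whether the actor is being destroyed.
; Health and stat change events are empty stubs.
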(event Custom|Event_OnHealthChanged)

(event Custom|Event_OnStatsChanged)

(event EventBeginPlay
  (Default|RecalculateStats (Variables|Default|GetStatsInventory)))

(event Collision|EventActorBeginOverlap
  (params (OtherActor :type Actor%20Object%20Reference)))

(event EventTick
  (params (DeltaSeconds :type Float%20%28single-precision%29)))

(fn ConstructionScript)

(fn Hit
  (params (Damages :type Array%20of%20S%20Damage%20Structures) (Attacker :type BP%20Base%20Character%20Object%20Reference) (First :type Boolean))
  (Default|Hit (Variables|Default|GetStatsInventory) Damages Attacker First))

(fn Kill
  (Default|ClearAllStatusEffects (Variables|Default|GetStatusEffectInventory)))

(fn IsDead
  (return (Game|IsActorBeingDestroyed)))