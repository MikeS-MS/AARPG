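; Base status effect that applies optional periodic damage to the player owning its status effect inventory, with an optional limited lifetime.
; Setup starts an expiry timer and, for ticking effects, divides damage values by tick time, hits immediately, repeats on a looping timer, then calls the empty PostSetup hook.
; Ticks skip dead players and damage through StatsInventory.
; Expiry removes the effect from its inventory, invalidates both timer handles and forces garbage collection.
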(event Custom|Setup
  (bind _stats (Variables|Default|GetStats))
  (Utilities|FlowControl|Sequence
    (:then_0
      (if (> (.time _stats) 0.0)
        (bind _returnvalue (Utilities|Time|SetTimerbyEvent (delegate Custom|DeleteEffect) (.time _stats)))
        (Variables|Default|SetDestructionTimer _returnvalue)))
    (:then_1
      (if (.ticks _stats)
        (CallFunction|TrimDamages)
        (CallFunction|Tick)
        (bind _returnvalue_2 (Utilities|Time|SetTimerbyFunctionName self "Tick" (.ticktime _stats) true))
        (Variables|Default|SetTimer _returnvalue_2)
        (CallFunction|PostSetup)))))

(event Custom|DeleteEffect
  (bind _owningstatuseffectinventory (Variables|Default|GetOwningStatusEffectInventory))
  (Utilities|IsValid _owningstatuseffectinventory
    (:Is%20Valid
      (Default|RemoveStatusEffect _owningstatuseffectinventory self)
      (Utilities|Time|InvalidateTimerHandle (Variables|Default|GetDestructionTimer))
      (Utilities|Time|InvalidateTimerHandle (Variables|Default|GetTimer))
      (Utilities|Platform|CollectGarbage))))

(fn Tick
  (bind _owningstatuseffectinventory (Variables|Default|GetOwningStatusEffectInventory))
  (bind _owningplayer (Variables|/Game/Blueprints/Characters/StatusEffects/BP_StatusEffectsInventory.BP_StatusEffectsInventory_C|GetOwningPlayer _owningstatuseffectinventory))
  (if (not (Default|IsDead _owningplayer))
    (Default|HitStatusEffect (Variables|/Game/Blueprints/Characters/BP_BaseCharacter.BP_BaseCharacter_C|GetStatsInventory _owningplayer) (Variables|Default|GetDamage) (Variables|Default|GetAttacker))))

(fn PostSetup)

(fn TrimDamages
  (bind _newdamage (LocalVariables|GetNewDamage))
  (for _array_element (Variables|Default|GetDamage)
    (Utilities|Array|Add _newdamage (Utilities|Struct|MakeS_Damage (.damagetype _array_element) (/ (.value _array_element) (.ticktime (Variables|Default|GetStats))) (.statuseffect _array_element))))
  (Variables|Default|SetDamage _newdamage))