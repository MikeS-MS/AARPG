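; Shield buff status effect that temporarily raises the owning player's damage resistances for as long as it exists.
; PreSetup copies the effect's Damage array into Resistances and adds it to the player's StatsInventory, and PreDestruction subtracts that stored copy.
; AccumulateStats rebuilds the stats struct, matching entries by damage type, so only resistance types already present on the player are adjusted.
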(fn PreSetup
  (bind _damage (Variables|Default|GetDamage))
  (|CallParentFunction)
  (Variables|Default|SetResistances _damage)
  (bind _owningstatuseffectinventory (Variables|Default|GetOwningStatusEffectInventory)
    (:then
      (bind _owningplayer (Variables|/Game/Blueprints/Characters/StatusEffects/BP_StatusEffectsInventory.BP_StatusEffectsInventory_C|GetOwningPlayer _owningstatuseffectinventory)
        (:then
          (CallFunction|AccumulateStats _damage (Variables|/Game/Blueprints/Characters/BP_BaseCharacter.BP_BaseCharacter_C|GetStatsInventory _owningplayer) true))
        (:else)))
    (:else)))

(fn PreDestruction
  (|CallParentFunction)
  (bind _owningstatuseffectinventory (Variables|Default|GetOwningStatusEffectInventory)
    (:then
      (bind _owningplayer (Variables|/Game/Blueprints/Characters/StatusEffects/BP_StatusEffectsInventory.BP_StatusEffectsInventory_C|GetOwningPlayer _owningstatuseffectinventory)
        (:then
          (CallFunction|AccumulateStats (Variables|Default|GetResistances) (Variables|/Game/Blueprints/Characters/BP_BaseCharacter.BP_BaseCharacter_C|GetStatsInventory _owningplayer) false))
        (:else)))
    (:else)))

(fn AccumulateStats
  (params (Resistances :type Array%20of%20S%20Damage%20Structures) (StatsInventory :type BP%20Stats%20Inventory%20Object%20Reference) (Additive :type Boolean))
  (bind _newresistances (LocalVariables|GetNewResistances))
  (Utilities|IsValid StatsInventory
    (:Is%20Valid
      (for _array_element (.resistances (Variables|/Game/Blueprints/Characters/Stats/BP_StatsInventory.BP_StatsInventory_C|GetStats StatsInventory))
        (LocalVariables|SetCurrentDamage "")
        (bind _array_element_2 (Utilities|Array|ForEachLoopwithBreak Resistances :!label _label)
          (:LoopBody
            (if (Utilities|Enum|Equal(Enum) (.damagetype _array_element) (.damagetype _array_element_2))
              (bind _output_get (LocalVariables|SetCurrentDamage (Utilities|Struct|MakeS_Damage (.damagetype _array_element_2) (.value _array_element_2) (.statuseffect _array_element_2))))
              (goto _label Break)))
          (:Completed
            (if Additive
              (Utilities|Array|Add _newresistances (Utilities|Struct|MakeS_Damage (.damagetype _array_element) (+ (.value _output_get) (.value _array_element)) (.statuseffect _array_element)))
              (else
                (Utilities|Array|Add _newresistances (Utilities|Struct|MakeS_Damage (.damagetype _array_element) (- (.value _array_element) (.value _output_get)) (.statuseffect _array_element))))))))
      (Variables|/Game/Blueprints/Characters/Stats/BP_StatsInventory.BP_StatsInventory_C|SetStats StatsInventory (Utilities|Struct|MakeS_Stats (.experience (Variables|/Game/Blueprints/Characters/Stats/BP_StatsInventory.BP_StatsInventory_C|GetStats StatsInventory)) (.maxhealth (Variables|/Game/Blueprints/Characters/Stats/BP_StatsInventory.BP_StatsInventory_C|GetStats StatsInventory)) (.thorns (Variables|/Game/Blueprints/Characters/Stats/BP_StatsInventory.BP_StatsInventory_C|GetStats StatsInventory)) (.damagetype (Variables|/Game/Blueprints/Characters/Stats/BP_StatsInventory.BP_StatsInventory_C|GetStats StatsInventory)) (LocalVariables|GetNewResistances) (.penetration (Variables|/Game/Blueprints/Characters/Stats/BP_StatsInventory.BP_StatsInventory_C|GetStats StatsInventory)))))))