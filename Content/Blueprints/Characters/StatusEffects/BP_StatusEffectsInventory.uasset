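; BP_StatusEffectsInventory tracks the status effects active on its owning BP_BaseCharacter.
; Adding an effect re-runs Setup on an existing one of that type, or constructs a new effect object from the game instance's StatusEffectManager stats, passing it the damage minus direct damage.
; Adds and removals recompute the owner's CanMove and CanAttack from the effects' movement and casting flags, and a clear function deletes every effect.
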(event EventBeginPlay
  (bind _asbp_rpggame_instance (Utilities|Casting|CastToBP_RPGGameInstance (Game|GetGameInstance)))
  (Variables|Default|SetStatusEffectManager (Variables|/Game/Blueprints/BP_RPGGameInstance.BP_RPGGameInstance_C|GetStatusEffectManager _asbp_rpggame_instance))
  (bind _asbp_base_character (Utilities|Casting|CastToBP_BaseCharacter (Components|GetOwner)))
  (Variables|Default|SetOwningPlayer _asbp_base_character))

(event EventTick
  (params (DeltaSeconds :type Float%20%28single-precision%29)))

(fn AddStatusEffect
  (params (StatusEffect :type E_StatusEffectNames%20Enum :default "NewEnumerator0") (Attacker :type BP%20Base%20Character%20Object%20Reference) (Damage :type Array%20of%20S%20Damage%20Structures))
  (bind _self self)
  (Utilities|AreValid Attacker (Variables|Default|GetOwningPlayer)
    (:Valid
      (bind (_exists _effect) (Utilitiy|EffectExists StatusEffect))
      (if _exists
        (Default|Setup _effect)
        (else
          (bind _statuseffectmanager (Utilities|GetStatusEffectManager)
            (:Valid
              (bind _stats (Default|GetStatsforStatusEffect _statuseffectmanager StatusEffect))
              (bind _trimmed (Utilitiy|RemoveDirectDamage Damage))
              (bind _returnvalue (Game|ConstructObjectfromClass (.classtoconstruct _stats) _self Attacker (.name _stats) _trimmed (.stats _stats) _self))
              (Utilities|Array|Add (Variables|Default|GetStatusEffects) _returnvalue)
              (Default|Setup _returnvalue)))))
      (Checks|UpdateCharacterValues))))

(fn EffectExists
  (params (StatusEffectType :type E_StatusEffectNames%20Enum :default "NewEnumerator0"))
  (for _array_element (Variables|Default|GetStatusEffects)
    (if (== (Variables|/Game/Blueprints/Characters/StatusEffects/BP_StatusEffect.BP_StatusEffect_C|GetStatusEffectName _array_element) StatusEffectType)
      (return true _array_element)))
  (return false 0))

(fn RemoveDirectDamage
  (params (Damages :type Array%20of%20S%20Damage%20Structures))
  (for _array_element Damages
    (if (not (Utilities|Enum|Equal(Enum) (.damagetype _array_element) "NewEnumerator0"))
      (Utilities|Array|Add (LocalVariables|GetTempTrimmed) (Utilities|Struct|MakeS_Damage (.damagetype _array_element) (.value _array_element) (.statuseffect _array_element)))))
  (return (LocalVariables|GetTempTrimmed)))

(fn UpdateCharacterValues
  (Utilities|IsValid (Variables|Default|GetOwningPlayer)
    (:Is%20Valid
      (Checks|CheckMovementStatusEffects)
      (Checks|CheckCastingStatusEffects))))

(fn CheckMovementStatusEffects
  (bind _owningplayer (Variables|Default|GetOwningPlayer))
  (for _array_element (Variables|Default|GetStatusEffects)
    (if (.affectsmovement (Variables|/Game/Blueprints/Characters/StatusEffects/BP_StatusEffect.BP_StatusEffect_C|GetStats _array_element))
      (Variables|/Game/Blueprints/Characters/BP_BaseCharacter.BP_BaseCharacter_C|SetCanMove _owningplayer false)
      (return)))
  (Variables|/Game/Blueprints/Characters/BP_BaseCharacter.BP_BaseCharacter_C|SetCanMove _owningplayer true))

(fn CheckCastingStatusEffects
  (bind _owningplayer (Variables|Default|GetOwningPlayer))
  (for _array_element (Variables|Default|GetStatusEffects)
    (if (.affectscasting (Variables|/Game/Blueprints/Characters/StatusEffects/BP_StatusEffect.BP_StatusEffect_C|GetStats _array_element))
      (Variables|/Game/Blueprints/Characters/BP_BaseCharacter.BP_BaseCharacter_C|SetCanAttack _owningplayer false)
      (return)))
  (Variables|/Game/Blueprints/Characters/BP_BaseCharacter.BP_BaseCharacter_C|SetCanAttack _owningplayer true))

(fn RemoveStatusEffect
  (params (StatusEffect :type BP%20Status%20Effect%20Object%20Reference))
  (Utilities|Array|RemoveItem (Variables|Default|GetStatusEffects) StatusEffect)
  (Checks|UpdateCharacterValues))

(fn ClearAllStatusEffects
  (for _array_element (Variables|Default|GetStatusEffects)
    (Default|DeleteEffect _array_element)))