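; BP_Spawner is a one-shot enemy spawner that fires when the RPG player character overlaps its trigger.
; It spawns each class in the EnemiesToSpawn map by its count at random points and yaws inside the SpawnZone actor's bounds.
; Each enemy gets a level within one of the player's, recalculated stats and ability damages, and a quest tag.
; It then sets Spawned and calls the empty OnEnemySpawned hook.
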(event OnComponentBeginOverlap(SpawnTrigger)
  (params (OverlappedComponent :type Primitive%20Component%20Object%20Reference) (OtherActor :type Actor%20Object%20Reference) (OtherComp :type Primitive%20Component%20Object%20Reference) (OtherBodyIndex :type Integer) (bFromSweep :type Boolean) (SweepResult :type Hit%20Result%20Structure%20%28by%20ref%29))
  (if (not (Variables|Default|GetSpawned))
    (bind _asbp_rpgplayer_character (Utilities|Casting|CastToBP_RPGPlayerCharacter OtherActor))
    (CallFunction|SpawnEnemies (Variables|/Game/Blueprints/Characters/Stats/BP_StatsInventory.BP_StatsInventory_C|GetLevel (Variables|/Game/Blueprints/Characters/BP_BaseCharacter.BP_BaseCharacter_C|GetStatsInventory _asbp_rpgplayer_character)))))

(fn ConstructionScript)

(fn SpawnEnemies
  (params (Level :type Integer))
  (bind _enemiestospawn (Variables|Default|GetEnemiesToSpawn))
  (bind _spawnzone (Variables|Default|GetSpawnZone))
  (bind (_origin _boxextent) (Collision|GetActorBounds _spawnzone false false))
  (bind _keys (Utilities|Map|Keys _enemiestospawn))
  (for _array_element _keys
    (for _index (range 1 (.Value (Utilities|Map|Find _enemiestospawn _array_element)))
      (bind _returnvalue (Game|SpawnActorfromClass _array_element (Math|Transform|MakeTransform (Math|Random|RandomPointinBoundingBox _origin _boxextent) (Math|Rotator|MakeRotator 0.0 0.0 (Math|Random|RandomFloatinRange 0.0 359.0)) "1,1,1") "AdjustIfPossibleButAlwaysSpawn" 0 0))
      (Variables|/Game/Blueprints/Characters/Stats/BP_StatsInventory.BP_StatsInventory_C|SetLevel (Variables|/Game/Blueprints/Characters/BP_BaseCharacter.BP_BaseCharacter_C|GetStatsInventory _returnvalue) (Math|Random|RandomIntegerinRange (- Level 1) (+ Level 1)))
      (Default|RecalculateStats (Variables|/Game/Blueprints/Characters/BP_BaseCharacter.BP_BaseCharacter_C|GetStatsInventory _returnvalue))
      (Default|CalculateAbilityDamages _returnvalue)
      (Variables|/Game/Blueprints/Characters/NPC/BP_Enemy.BP_Enemy_C|SetQuestTag _returnvalue (Variables|Default|GetEnemyQuestTag))))
  (Variables|Default|SetSpawned true)
  (CallFunction|OnEnemySpawned))

(fn OnEnemySpawned)