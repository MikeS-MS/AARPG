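; BP_Enemy is a base enemy character that spawns its controller, gets ability stats from the game instance's EnemyAbilityManager, and leaves Attack as a stub returning false.
; A HomingArea overlap registers it as NearestEnemy on non-enemy projectiles.
; Its HealthArea shows a health bar rotated toward the player's camera, refreshed on health or stat changes.
; Kill destroys its inventory components and actor, then forces garbage collection.
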(event OnComponentBeginOverlap(HealthArea)
  (params (OverlappedComponent :type Primitive%20Component%20Object%20Reference) (OtherActor :type Actor%20Object%20Reference) (OtherComp :type Primitive%20Component%20Object%20Reference) (OtherBodyIndex :type Integer) (bFromSweep :type Boolean) (SweepResult :type Hit%20Result%20Structure%20%28by%20ref%29))
  (bind _health (Variables|Default|GetHealth))
  (bind _asbp_rpgplayer_character (Utilities|Casting|CastToBP_RPGPlayerCharacter OtherActor))
  (Variables|/Game/Blueprints/Characters/NPC/BPW_HealthComponent.BPW_HealthComponent_C|SetTargetToRotateTo _health (Variables|/Game/Blueprints/Characters/Player/BP_RPGPlayerCharacter.BP_RPGPlayerCharacter_C|GetFollowCamera _asbp_rpgplayer_character))
  (Rendering|SetVisibility _health true true))

(event OnComponentBeginOverlap(HomingArea)
  (params (OverlappedComponent :type Primitive%20Component%20Object%20Reference) (OtherActor :type Actor%20Object%20Reference) (OtherComp :type Primitive%20Component%20Object%20Reference) (OtherBodyIndex :type Integer) (bFromSweep :type Boolean) (SweepResult :type Hit%20Result%20Structure%20%28by%20ref%29))
  (bind _projectile (Utilities|CasttoProjectile OtherActor OtherComp)
    (:Is
      (if (not (Variables|/Game/Blueprints/Characters/Player/Abilities/BPP_BaseProjectile.BPP_BaseProjectile_C|GetEnemyProjectile _projectile))
        (Variables|/Game/Blueprints/Characters/Player/Abilities/BPP_BaseProjectile.BPP_BaseProjectile_C|SetNearestEnemy _projectile self)))))

(event OnComponentEndOverlap(HomingArea)
  (params (OverlappedComponent :type Primitive%20Component%20Object%20Reference) (OtherActor :type Actor%20Object%20Reference) (OtherComp :type Primitive%20Component%20Object%20Reference) (OtherBodyIndex :type Integer))
  (bind _projectile (Utilities|CasttoProjectile OtherActor OtherComp)
    (:Is
      (if (and (== (Variables|/Game/Blueprints/Characters/Player/Abilities/BPP_BaseProjectile.BPP_BaseProjectile_C|GetNearestEnemy _projectile) self) (not (Variables|/Game/Blueprints/Characters/Player/Abilities/BPP_BaseProjectile.BPP_BaseProjectile_C|GetEnemyProjectile _projectile)))
        (Variables|/Game/Blueprints/Characters/Player/Abilities/BPP_BaseProjectile.BPP_BaseProjectile_C|SetNearestEnemy _projectile 0)))))

(event OnComponentEndOverlap(HealthArea)
  (params (OverlappedComponent :type Primitive%20Component%20Object%20Reference) (OtherActor :type Actor%20Object%20Reference) (OtherComp :type Primitive%20Component%20Object%20Reference) (OtherBodyIndex :type Integer))
  (bind _health (Variables|Default|GetHealth))
  (Utilities|Casting|CastToBP_RPGPlayerCharacter OtherActor)
  (Rendering|SetVisibility _health false true)
  (Variables|/Game/Blueprints/Characters/NPC/BPW_HealthComponent.BPW_HealthComponent_C|SetTargetToRotateTo _health 0))

(event EventBeginPlay
  (|CallParentFunction)
  (Utilities|FlowControl|Sequence
    (:then_0
      (bind _aswbp_health_bar (Utilities|Casting|CastToWBP_HealthBar (UserInterface|GetUserWidgetObject (Variables|Default|GetHealth))))
      (Variables|/Game/UI/WBP_HealthBar.WBP_HealthBar_C|SetEnemy _aswbp_health_bar self)
      (bind _output_get (Variables|Instances|SetHealthWidget _aswbp_health_bar))
      (Default|UpdateValues _output_get))
    (:then_1
      (bind _asbp_rpggame_instance (Utilities|Casting|CastToBP_RPGGameInstance (Game|GetGameInstance)))
      (Variables|Instances|SetEnemyAbilityManager (Variables|/Game/Blueprints/BP_RPGGameInstance.BP_RPGGameInstance_C|GetEnemyAbilityManager _asbp_rpggame_instance))
      (CallFunction|CalculateAbilityDamages))
    (:then_2
      (Pawn|SpawnDefaultController))))

(event Collision|EventActorBeginOverlap
  (params (OtherActor :type Actor%20Object%20Reference)))

(event EventTick
  (params (DeltaSeconds :type Float%20%28single-precision%29))
  (|CallParentFunction DeltaSeconds))

(event EventEventonHealthChanged
  (bind _healthwidget (Variables|Instances|GetHealthWidget))
  (Utilities|IsValid _healthwidget
    (:Is%20Valid
      (Default|UpdateValues _healthwidget))))

(event EventEventonStatsChanged
  (bind _healthwidget (Variables|Instances|GetHealthWidget))
  (Utilities|IsValid _healthwidget
    (:Is%20Valid
      (Default|UpdateValues _healthwidget))))

(fn ConstructionScript)

(fn Kill
  (|CallParentFunction)
  (Components|DestroyComponent (Variables|Default|GetStatsInventory))
  (Components|DestroyComponent (Variables|Default|GetStatusEffectInventory))
  (Actor|DestroyActor)
  (Utilities|Platform|CollectGarbage))

(fn Attack
  (params (Target :type BP%20Base%20Character%20Object%20Reference))
  (return false))

(fn CalculateAbilityDamages
  (Variables|Ability|SetAbilityStats (Default|GetStats (Variables|Instances|GetEnemyAbilityManager) (Variables|Ability|GetAbilityType) self)))