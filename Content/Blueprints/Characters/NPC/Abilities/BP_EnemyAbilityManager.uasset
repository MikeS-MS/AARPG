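; Enemy ability manager that resolves an ability's damage and extra stats for a given NPC from base and per-level stat maps.
; GetStats returns extra stats unscaled, and raw base damage when no per-level data exists.
; Otherwise, AccumulateDamageLists pairs entries by index, scaling base plus level growth by the enemy's damage and StatsManager type multipliers.
; Entries with mismatched damage type or status effect, or missing multipliers, are dropped.
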(fn AccumulateDamageLists
  (params (Base :type Array%20of%20S%20Damage%20Structures) (PerLevel :type Array%20of%20S%20Damage%20Structures) (Level :type Integer) (Enemy :type BP%20Enemy%20Object%20Reference))
  (bind _temp (LocalVariables|GetTemp))
  (bind _statsinventory (Variables|/Game/Blueprints/Characters/BP_BaseCharacter.BP_BaseCharacter_C|GetStatsInventory Enemy))
  (bind _statsmanager (Variables|/Game/Blueprints/Characters/Stats/BP_StatsInventory.BP_StatsInventory_C|GetStatsManager _statsinventory))
  (bind _stats (Variables|/Game/Blueprints/Characters/Stats/BP_StatsInventory.BP_StatsInventory_C|GetStats _statsinventory))
  (for (_array_element _array_index) Base
    (if (Math|Boolean|ANDBoolean (Utilities|Enum|Equal(Enum) (.damagetype _array_element) (.damagetype (Utilities|Array|Get(acopy) PerLevel _array_index))) (Math|Boolean|Equal(Boolean) (.statuseffect _array_element) (.statuseffect (Utilities|Array|Get(acopy) PerLevel _array_index))) (.Found (Default|GetDamagesEntry _statsmanager (.damagetype _array_element))) (.Found (Default|GetCharacterDamageTypeValue _statsmanager (.damagetype (.damagetype _stats)) (.DamageTypeMultipliers (Default|GetDamagesEntry _statsmanager (.damagetype _array_element))))))
      (Utilities|Array|Add _temp (Utilities|Struct|MakeS_Damage (.damagetype (Utilities|Array|Get(acopy) PerLevel _array_index)) (* (* (* (.Value (Default|GetDamagesEntry _statsmanager (.damagetype _array_element))) (.Value (Default|GetCharacterDamageTypeValue _statsmanager (.damagetype (.damagetype _stats)) (.DamageTypeMultipliers (Default|GetDamagesEntry _statsmanager (.damagetype _array_element)))))) (.damage (.damagetype _stats))) (+ (.value _array_element) (* Level (.value (Utilities|Array|Get(acopy) PerLevel _array_index))))) (.statuseffect (Utilities|Array|Get(acopy) PerLevel _array_index))))))
  (return _temp))

(fn GetStats
  (params (Ability :type E_EnemyAbilityType%20Enum :default "NewEnumerator0") (Character :type BP%20Enemy%20Object%20Reference))
  (bind _baseabilitystats (Variables|Default|GetBaseAbilityStats))
  (bind _perlevelabilitystats (Variables|Default|GetPerLevelAbilityStats))
  (bind (_value _returnvalue) (Utilities|Map|Find _perlevelabilitystats Ability))
  (bind (_value_2 _returnvalue_2) (Utilities|Map|Find _baseabilitystats Ability))
  (if _returnvalue_2
    (if _returnvalue
      (return (Utilities|Struct|MakeS_AbilityDamagesAndStats (CallFunction|AccumulateDamageLists (.damage _value_2) (.damage _value) (Variables|/Game/Blueprints/Characters/Stats/BP_StatsInventory.BP_StatsInventory_C|GetLevel (Variables|/Game/Blueprints/Characters/BP_BaseCharacter.BP_BaseCharacter_C|GetStatsInventory Character)) Character) (.extrastats _value_2)))
      (else
        (return (Utilities|Struct|MakeS_AbilityDamagesAndStats (.damage _value_2) (.extrastats _value_2)))))
    (else
      (return ""))))