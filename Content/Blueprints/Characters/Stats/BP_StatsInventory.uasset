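; Character stats component for BP_BaseCharacter owners that handles levels, health and incoming damage.
; RecalculateStats builds stats from the game instance's StatsManager by NPC type, adding level-scaled values to base ones; LevelUp reruns it, refilling health.
; Hits divide damage by resistance, offset by attacker penetration, and kill at zero health.
; Poison hits add a status effect, whose damage HitStatusEffect handles; Thorns reflects first hits only, preventing loops.
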(event EventBeginPlay
  (bind _asbp_rpggame_instance (Utilities|Casting|CastToBP_RPGGameInstance (Game|GetGameInstance)))
  (Variables|Instances|SetStatsManager (Variables|/Game/Blueprints/BP_RPGGameInstance.BP_RPGGameInstance_C|GetStatsManager _asbp_rpggame_instance))
  (bind _asbp_base_character (Utilities|Casting|CastToBP_BaseCharacter (Components|GetOwner)))
  (Variables|Instances|SetCharacter _asbp_base_character))

(event EventTick
  (params (DeltaSeconds :type Float%20%28single-precision%29)))

(fn RecalculateStats
  (bind _statsmanager (Variables|Instances|GetStatsManager))
  (bind _character (Variables|Instances|GetCharacter))
  (bind _level (Variables|Stats|GetLevel))
  (bind _basestats (Variables|/Game/Blueprints/Characters/Stats/BP_StatsManager.BP_StatsManager_C|GetBaseStats _statsmanager))
  (bind _npctype (Variables|/Game/Blueprints/Characters/BP_BaseCharacter.BP_BaseCharacter_C|GetNPCType _character))
  (bind _perlevelstats (Variables|/Game/Blueprints/Characters/Stats/BP_StatsManager.BP_StatsManager_C|GetPerLevelStats _statsmanager))
  (bind (_found _stats) (Default|GetStatsEntry _statsmanager _perlevelstats _npctype))
  (bind (_found_2 _stats_2) (Default|GetStatsEntry _statsmanager _basestats _npctype))
  (if (and _found_2 _found)
    (bind _output_get (Variables|Stats|SetStats (Utilities|Struct|MakeS_Stats 1.2e+03 (+ (.maxhealth _stats_2) (* _level (.maxhealth _stats))) (+ (.thorns _stats_2) (* _level (.thorns _stats))) (Utilities|Struct|MakeS_CharacterDamageType (.damagetype (.damagetype _stats_2)) (+ (.damage (.damagetype _stats_2)) (* _level (.damage (.damagetype _stats))))) (CallFunction|AccumulateStatLists (.resistances _stats_2) (.resistances _stats)) (CallFunction|AccumulateStatLists (.penetration _stats_2) (.penetration _stats)))))
    (Variables|Stats|SetMaxExperience (+ (.experience _stats_2) (* _level (.experience _stats))))
    (Variables|Stats|SetCurrentHealth (.maxhealth _output_get))))

(fn AddXP
  (params (XP :type Float%20%28single-precision%29))
  (if (not (Variables|Stats|GetReachedMaxLevel))
    (if (>= (+ (Variables|Stats|GetCurrentExperience) XP) (Variables|Stats|GetMaxExperience))
      (bind _leveledup (CallFunction|LevelUp))
      (if _leveledup
        (Variables|Stats|SetCurrentExperience 0.0)))))

(fn LevelUp
  (if (>= (+ (Variables|Stats|GetLevel) 1) (Variables|Stats|GetMaxLevel))
    (Variables|Stats|SetLevel (Variables|Stats|GetMaxLevel))
    (Variables|Stats|SetCurrentExperience (Variables|Stats|GetMaxExperience))
    (Variables|Stats|SetReachedMaxLevel true)
    (return false)
    (else
      (Variables|Stats|SetLevel (+ (Variables|Stats|GetLevel) 1))
      (CallFunction|RecalculateStats)
      (Variables|Stats|SetCurrentHealth (.maxhealth (Variables|Stats|GetStats)))
      (return true))))

(fn Hit
  (params (Damage :type Array%20of%20S%20Damage%20Structures) (Attacker :type BP%20Base%20Character%20Object%20Reference) (First :type Boolean))
  (bind _stats (Variables|Stats|GetStats))
  (bind _character (Variables|Instances|GetCharacter))
  (bind _thornsdamage (LocalVariables|GetThornsDamage))
  (for _array_element Damage
    (Utilities|FlowControl|Sequence
      (:then_0
        (switch Utilities|FlowControl|Switch|SwitchonE_DamageType (.damagetype _array_element)
          (:NewEnumerator7
            (Default|AddStatusEffect (Variables|/Game/Blueprints/Characters/BP_BaseCharacter.BP_BaseCharacter_C|GetStatusEffectInventory _character) "NewEnumerator4" Attacker Damage))))
      (:then_1
        (if (not (.statuseffect _array_element))
          (bind _newdamage (CallFunction|GetCalculatedDamage (Utilities|Struct|MakeS_Damage (.damagetype _array_element) (.value _array_element) false) (Variables|/Game/Blueprints/Characters/BP_BaseCharacter.BP_BaseCharacter_C|GetStatsInventory Attacker)))
          (if (>= _newdamage 0.0)
            (LocalVariables|SetAccumulatedDamage (+ _newdamage (LocalVariables|GetAccumulatedDamage))))))))
  (bind _output_get (LocalVariables|SetNewHealth (- (Variables|Stats|GetCurrentHealth) (LocalVariables|GetAccumulatedDamage))))
  (if (<= _output_get 0.0)
    (Variables|Stats|SetCurrentHealth 0.0)
    (Default|Kill _character)
    (else
      (Variables|Stats|SetCurrentHealth _output_get)
      (if (and (> (.thorns _stats) 0.0) First)
        (for _array_element_2 Damage
          (Utilities|Array|Add _thornsdamage (Utilities|Struct|MakeS_Damage (.damagetype _array_element_2) (* (.value _array_element_2) (.thorns _stats)) false)))
        (Default|Attack Attacker _thornsdamage _character false)))))

(fn HitStatusEffect
  (params (Damage :type Array%20of%20S%20Damage%20Structures) (Attacker :type BP%20Base%20Character%20Object%20Reference))
  (if (and (not (Game|IsActorBeingDestroyed Attacker)) (not (Game|IsActorBeingDestroyed (Variables|Instances|GetCharacter))))
    (for _array_element Damage
      (bind _newdamage (CallFunction|GetCalculatedDamage (Utilities|Struct|MakeS_Damage (.damagetype _array_element) (.value _array_element) (.statuseffect _array_element)) (Variables|/Game/Blueprints/Characters/BP_BaseCharacter.BP_BaseCharacter_C|GetStatsInventory Attacker)))
      (if (>= _newdamage 0.0)
        (LocalVariables|SetAccumulatedDamage (+ _newdamage (LocalVariables|GetAccumulatedDamage)))))
    (bind _output_get (LocalVariables|SetNewHealth (- (Variables|Stats|GetCurrentHealth) (LocalVariables|GetAccumulatedDamage))))
    (if (<= _output_get 0.0)
      (Variables|Stats|SetCurrentHealth 0.0)
      (Default|Kill (Variables|Instances|GetCharacter))
      (else
        (Variables|Stats|SetCurrentHealth _output_get)))))

(fn GetCalculatedDamage
  (params (Damage :type S%20Damage%20Structure) (AttackerStatsInventory :type BP%20Stats%20Inventory%20Object%20Reference))
  (bind _stats (Variables|Stats|GetStats))
  (bind _stats_2 (Variables|BP_StatsInventory_C|GetStats AttackerStatsInventory))
  (bind (_value _found) (CallFunction|GetValue (.penetration _stats_2) (.damagetype Damage)))
  (bind (_value_2 _found_2) (CallFunction|GetValue (.resistances _stats) (.damagetype Damage)))
  (bind _returnvalue (/ (.value Damage) _value_2))
  (bind _returnvalue_2 (- _value_2 _value))
  (if _found_2
    (if _found
      (if (< _returnvalue_2 1.0)
        (return _returnvalue)
        (else
          (return (/ (.value Damage) _returnvalue_2))))
      (else
        (return _returnvalue)))
    (else
      (return (.value Damage)))))

(fn GetValue
  (params (List :type Array%20of%20S%20Damage%20Structures) (EntryType :type E_DamageType%20Enum :default "NewEnumerator8"))
  (for _array_element List
    (if (== (.DamageType (Utilities|Struct|BreakS_Damage _array_element)) EntryType)
      (return (.Value (Utilities|Struct|BreakS_Damage _array_element)) true)))
  (return 0.0 false))

(fn AccumulateStatLists
  (params (Base :type Array%20of%20S%20Damage%20Structures) (PerLevel :type Array%20of%20S%20Damage%20Structures))
  (bind _result (LocalVariables|GetResult))
  (for (_array_element _array_index) Base
    (if (and (Utilities|Enum|Equal(Enum) (.damagetype _array_element) (.damagetype (Utilities|Array|Get(acopy) PerLevel _array_index))) (Math|Boolean|Equal(Boolean) (.statuseffect _array_element) (.statuseffect (Utilities|Array|Get(acopy) PerLevel _array_index))))
      (Utilities|Array|Add _result (Utilities|Struct|MakeS_Damage (.damagetype (Utilities|Array|Get(acopy) PerLevel _array_index)) (+ (.value _array_element) (* (Variables|Stats|GetLevel) (.value (Utilities|Array|Get(acopy) PerLevel _array_index)))) (.statuseffect (Utilities|Array|Get(acopy) PerLevel _array_index))))))
  (return _result))