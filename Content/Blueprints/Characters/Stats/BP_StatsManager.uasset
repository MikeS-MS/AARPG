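; BP_StatsManager provides lookup functions for character stats and damage-type data.
; Each function linearly searches an array of structs and returns the first match with a Found flag.
; GetStatsEntry maps an NPC type to stats and GetCharacterDamageTypeValue maps a damage type to damage, both from passed-in lists.
; GetDamageEntry searches the DamageMultipliers variable for a damage type's value, status effect and multipliers.
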(fn GetStatsEntry
  (params (List :type Array%20of%20S%20Character%20Stats%20Structures) (Type :type E_NPCType%20Enum :default "NewEnumerator0"))
  (for _array_element List
    (if (== (.npctype _array_element) Type)
      (return true (.stats _array_element))))
  (return false ""))

(fn GetDamageEntry
  (params (DamageType :type E_DamageType%20Enum :default "NewEnumerator6"))
  (for _array_element (Variables|Default|GetDamageMultipliers)
    (if (Utilities|Enum|Equal(Enum) (.damagetype (.damagetype _array_element)) DamageType)
      (return true (.value (.damagetype _array_element)) (.statuseffect (.damagetype _array_element)) (.damagetypemultipliers _array_element))))
  (return false 0.0 false 0))

(fn GetCharacterDamageTypeValue
  (params (CharacterDamageType :type E_CharacterDamageType%20Enum :default "NewEnumerator0") (List :type Array%20of%20S%20Character%20Damage%20Type%20Structures))
  (for _array_element List
    (if (Utilities|Enum|Equal(Enum) (.damagetype _array_element) CharacterDamageType)
      (return true (.damage _array_element))))
  (return false 0.0))