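; RPG game mode that handles player death and respawning.
; BindPlayer hooks the player character's death event, which unpossesses the controller and starts a three-second timer.
; RespawnPlayer then finds the BP_RespawnPoint nearest the stored character and delegates spawning to it, creating a new respawn point if none is valid.
; BeginPlay is empty, so nothing in this graph calls BindPlayer.
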(event Custom|PlayerDead
  (bind _asbp_rpgplayer_character (Utilities|Casting|CastToBP_RPGPlayerCharacter (Game|GetPlayerCharacter 0)))
  (Variables|Default|SetPlayer _asbp_rpgplayer_character)
  (Pawn|UnPossess (Game|GetPlayerController 0))
  (Utilities|Time|SetTimerbyFunctionName 0 "RespawnPlayer" 3.0))

(event Custom|BindDeathEvent
  (params (Player :type BP%20RPG%20Player%20Character%20Object%20Reference))
  (EventDispatchers|AssignPlayerDead Player (delegate Custom|PlayerDead)))

(event Custom|BindPlayer
  (bind _asbp_rpgplayer_character (Utilities|Casting|CastToBP_RPGPlayerCharacter (Game|GetPlayerCharacter 0)))
  (CallFunction|BindDeathEvent _asbp_rpgplayer_character))

(event EventBeginPlay)

(fn ConstructionScript)

(fn RespawnPlayer
  (bind _player (Variables|Default|GetPlayer))
  (bind _player_2 (Variables|Default|GetPlayer))
  (bind _returnvalue (Transformation|GetActorLocation _player_2))
  (bind _outactors (Actor|GetAllActorsOfClass "/Game/Blueprints/Characters/Player/BP_RespawnPoint.BP_RespawnPoint_C"))
  (Utilities|IsValid (Utilities|Array|Get(acopy) _outactors)
    (:Is%20Valid
      (LocalVariables|SetClosestDistance (Math|Vector|Distance(Vector) (Transformation|GetActorLocation (Utilities|Array|Get(acopy) _outactors)) _returnvalue))
      (LocalVariables|SetClosestPoint (Utilities|Array|Get(acopy) _outactors)))
    (:Is%20Not%20Valid
      (bind _output_get (LocalVariables|SetClosestDistance 1e+08))))
  (for _array_element _outactors
    (if (< (Math|Vector|Distance(Vector) (Transformation|GetActorLocation _array_element) _returnvalue) _output_get)
      (LocalVariables|SetClosestDistance (Math|Vector|Distance(Vector) (Transformation|GetActorLocation _array_element) _returnvalue))
      (LocalVariables|SetClosestPoint _array_element)))
  (Utilities|IsValid (LocalVariables|GetClosestPoint)
    (:Is%20Valid
      (Default|SpawnPlayer (LocalVariables|GetClosestPoint) _player))
    (:Is%20Not%20Valid
      (bind _returnvalue_2 (Game|SpawnActorfromClass "/Game/Blueprints/Characters/Player/BP_RespawnPoint.BP_RespawnPoint_C" (Math|Transform|MakeTransform "0, 0, 0" "0, 0, 0" "1,1,1") "Undefined" 0 0))
      (Default|SpawnPlayer _returnvalue_2 _player))))