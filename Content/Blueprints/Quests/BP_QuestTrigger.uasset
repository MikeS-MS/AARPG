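; Quest trigger actor that fires quest logic when the RPG player character enters its box.
; The overlap calls QuestTrigger on its QuestComponent and, on success, fires the pickup event on a child BP_QuestItemPickup actor.
; The construction script copies the actor's quest settings into the component and its hide-on-trigger flag into the pickup.
; Functions to activate, complete and update item trackers through GameQuestSubsystem are defined but not called within this Blueprint.
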(event OnComponentBeginOverlap(Box)
  (params (OverlappedComponent :type Primitive%20Component%20Object%20Reference) (OtherActor :type Actor%20Object%20Reference) (OtherComp :type Primitive%20Component%20Object%20Reference) (OtherBodyIndex :type Integer) (bFromSweep :type Boolean) (SweepResult :type Hit%20Result%20Structure%20%28by%20ref%29))
  (Utilities|Casting|CastToBP_RPGPlayerCharacter OtherActor)
  (bind _successful (Default|QuestTrigger (Variables|Default|GetQuestComponent)))
  (if _successful
    (CallFunction|PickupItem)))

(fn ConstructionScript
  (bind _questcomponent (Variables|Default|GetQuestComponent))
  (Utilities|FlowControl|Sequence
    (:then_0
      (bind _asbp_quest_item_pickup (Utilities|Casting|CastToBP_QuestItemPickup (Variables|/Script/Engine.ChildActorComponent|GetChildActor (Variables|Default|GetBP_PickupItem))))
      (Variables|/Game/Blueprints/Quests/BP_QuestItemPickup.BP_QuestItemPickup_C|SetbHideItemPickupOnTrigger _asbp_quest_item_pickup (Variables|Default|GetbHideItemOnTrigger)))
    (:then_1
      (Variables|/Game/Blueprints/Quests/QuestTriggerComponent.QuestTriggerComponent_C|SetItems _questcomponent (Variables|Default|GetItems))
      (Variables|/Game/Blueprints/Quests/QuestTriggerComponent.QuestTriggerComponent_C|SetbExpireOnTrigger _questcomponent (Variables|Default|GetbExpireOnTrigger))
      (Variables|/Game/Blueprints/Quests/QuestTriggerComponent.QuestTriggerComponent_C|SetQuestID _questcomponent (Variables|Default|GetQuestID))
      (Variables|/Game/Blueprints/Quests/QuestTriggerComponent.QuestTriggerComponent_C|SetTriggerType _questcomponent (Variables|Default|GetTriggerType)))))

(fn CompleteQuest
  (bind _questid (Variables|Default|GetQuestID))
  (Class|GameQuestSubsystem|CompleteQuest (Subsystems|GetGameQuestSubsystem) _questid)
  (Development|PrintString (Utilities|String|Append "Quest with ID completed: " (Utilities|String|ToString(Integer) _questid))))

(fn ActivateQuest
  (bind _questid (Variables|Default|GetQuestID))
  (Class|GameQuestSubsystem|ActivateQuest (Subsystems|GetGameQuestSubsystem) _questid)
  (Development|PrintString (Utilities|String|Append "Quest with ID activated: " (Utilities|String|ToString(Integer) _questid))))

(fn UpdateQuestItems
  (bind _items (Variables|Default|GetItems))
  (bind _keys (Utilities|Map|Keys _items))
  (for _array_element _keys
    (if (.ReturnValue (Utilities|Map|Find _items _array_element))
      (Class|GameQuestSubsystem|UpdateQuestItemTracker (Subsystems|GetGameQuestSubsystem) _array_element (.Value (Utilities|Map|Find _items _array_element)))))
  (Development|PrintString "Updated all quest requirements."))

(fn PickupItem
  (bind _asbp_quest_item_pickup (Utilities|Casting|CastToBP_QuestItemPickup (Variables|/Script/Engine.ChildActorComponent|GetChildActor (Variables|Default|GetBP_PickupItem))))
  (Default|PickupItemEvent _asbp_quest_item_pickup))