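; QuestTestGameMode is a test game mode that feeds sample quests into the game's quest subsystem.
; LoadQuestsInSub counts the rows of DT_QuestsSample, looks each up by a numeric name from 1 to that count, and collects the quests found.
; It passes the array to GameQuestSubsystem's LoadQuests and prints a confirmation.
; BeginPlay is empty, and nothing in this Blueprint calls the load function.
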(event EventBeginPlay)

(fn ConstructionScript
  (|CallParentFunction))

(fn LoadQuestsinSub
  (Utilities|FlowControl|Sequence
    (:then_0
      (bind _outrownames (DataTable|GetDataTableRowNames "/Game/Blueprints/Quests/DT_QuestsSample.DT_QuestsSample"))
      (LocalVariables|SetQuestRowNames _outrownames)
      (LocalVariables|SetQuestNum (Utilities|Array|Length _outrownames)))
    (:then_1
      (for _index (range 1 (LocalVariables|GetQuestNum))
        (bind _returnvalue (Utilities|GetDataTableRow "/Game/Blueprints/Quests/DT_QuestsSample.DT_QuestsSample" (Utilities|String|StringToName (Utilities|String|ToString(Integer) _index)))
          (:then
            (Utilities|Array|Add (LocalVariables|GetQuests) (Utilities|Struct|BreakFQuestRow _returnvalue)))))
      (Class|GameQuestSubsystem|LoadQuests (Subsystems|GetGameQuestSubsystem) (LocalVariables|GetQuests))
      (Development|PrintString "Loaded quests from sample"))))