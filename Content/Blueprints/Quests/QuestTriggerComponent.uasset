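; Quest trigger component that completes, activates or updates item requirements for a quest through the game quest subsystem.
; QuestTrigger accepts only an RPG player character instigator, branches on TriggerType, then marks itself expired so it fires once.
; The item update loops over the Items map and pushes each item name and quantity to the subsystem's tracker.
; Each action also prints debug strings.
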(fn CompleteQuest
  (bind _questid (Variables|Default|GetQuestID))
  (Class|GameQuestSubsystem|CompleteQuest (Subsystems|GetGameQuestSubsystem) _questid)
  (Development|PrintString (Utilities|String|Append "Quest with ID completed: " (Utilities|String|ToString(Integer) _questid))))

(fn ActivateQuest
  (bind _questid (Variables|Default|GetQuestID))
  (Class|GameQuestSubsystem|ActivateQuest (Subsystems|GetGameQuestSubsystem) _questid)
  (Development|PrintString (Utilities|String|Append "Quest with ID activated: " (Utilities|String|ToString(Integer) _questid))))

(fn UpdateQuestItems
  (bind _items (Variables|Default|GetItems))
  (bind _keys (Utilities|Map|Keys _items))
  (for _array_element _keys
    (if (.ReturnValue (Utilities|Map|Find _items _array_element))
      (Class|GameQuestSubsystem|UpdateQuestItemTracker (Subsystems|GetGameQuestSubsystem) _array_element (.Value (Utilities|Map|Find _items _array_element)))))
  (Development|PrintString "Updated all quest requirements."))

(fn QuestTrigger
  (params (Instigator :type Object%20Object%20Reference))
  (if (not (Variables|Default|GetbExpired))
    (Utilities|Casting|CastToBP_RPGPlayerCharacter Instigator)
    (switch Utilities|FlowControl|Switch|SwitchonEQuestTriggerType (Variables|Default|GetTriggerType)
      (:NewEnumerator0
        (CallFunction|CompleteQuest))
      (:NewEnumerator1
        (CallFunction|ActivateQuest))
      (:NewEnumerator2
        (CallFunction|UpdateQuestItems)))
    (Variables|Default|SetbExpired true)
    (Development|PrintString "Hello")))