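; AI controller for enemy NPCs that runs the BT_Enemy behavior tree and feeds it target state through the blackboard.
; BeginPlay hardcodes the NPC type, logged as archer, and binds to the player's death event.
; AI perception sets TargetActor on sighting player-tagged actors and clears it on lost perception or player death.
; UpdateTargetActorKey forces targeting when hit; both targeting paths copy the target's dead flag to TargetDead.
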(event OnTargetPerceptionUpdated(AIPerception)
  (params (Actor :type Actor%20Object%20Reference) (Stimulus :type AI%20Stimulus%20Structure))
  (bind _returnvalue (Utilities|Name|MakeLiteralName "TargetActor"))
  (bind _blackboard (Variables|Default|GetBlackboard))
  ;[0 0 0] When the perception component gains or loses sight this event fires and we deduce from the Stimulus struct which one it is
  (if (Utilities|Array|ContainsItem (Variables|/Script/Engine.Actor|GetTags Actor) "player")
    (bind _asbp_base_character (Utilities|Casting|CastToBP_BaseCharacter Actor))
    (CallFunction|SetDeadKey (Variables|/Game/Blueprints/Characters/BP_BaseCharacter.BP_BaseCharacter_C|GetDead _asbp_base_character))
    (Variables|Default|SetTargetActor Actor)
    (if (.bSuccessfullySensed (Utilities|Struct|BreakAIStimulus Stimulus))
      (AI|Components|Blackboard|SetValueasObject _blackboard _returnvalue (Variables|Default|GetTargetActor))
      (Development|PrintString "Acquired enemy")
      (else
        (AI|Components|Blackboard|SetValueasObject _blackboard _returnvalue 0)
        (Development|PrintString "Lost enemy")))))

(event Custom|PlayerDead_Event_0
  ;[0 0 0] When the perception component gains or loses sight this event fires and we deduce from the Stimulus struct which one it is
  (AI|Components|Blackboard|SetValueasObject (Variables|Default|GetBlackboard) (Utilities|Name|MakeLiteralName "TargetActor") 0)
  (Development|PrintString "Lost enemy"))

(event Custom|SetDeadKey
  (params (PlayerDead :type Boolean))
  (AI|Components|Blackboard|SetValueasBool (Variables|Default|GetBlackboard) (Utilities|Name|MakeLiteralName "TargetDead") PlayerDead))

(event Custom|UpdateTargetActorKey
  (params (TargetActor :type Actor%20Object%20Reference))
  ;[0 0 0] Used when player hits an enemy and the enemy targets them automatically
  (bind _output_get (Variables|Default|SetTargetActor TargetActor))
  (AI|Components|Blackboard|SetValueasObject (Variables|Default|GetBlackboard) (Utilities|Name|MakeLiteralName "TargetActor") _output_get)
  (bind _asbp_base_character (Utilities|Casting|CastToBP_BaseCharacter _output_get))
  (CallFunction|SetDeadKey (Variables|/Game/Blueprints/Characters/BP_BaseCharacter.BP_BaseCharacter_C|GetDead _asbp_base_character)))

(event EventBeginPlay
  ;[0 0 0] Runs the behaviour tree for the enemy BT and sets the NPC Type
  (AI|RunBehaviorTree "/Game/Blueprints/AI/BT_Enemy.BT_Enemy")
  (AI|Components|Blackboard|SetValueasEnum (Variables|Default|GetBlackboard) (Utilities|Name|MakeLiteralName "NPCType") (Utilities|Enum|LiteralenumE_NPCType "NewEnumerator2"))
  (Development|PrintString "Setting default NPC type to archer [hardcoded]" false)
  (bind _asbp_rpgplayer_character (Utilities|Casting|CastToBP_RPGPlayerCharacter (Pawn|GetControlledPawn (Game|GetPlayerController 0))))
  (EventDispatchers|AssignPlayerDead _asbp_rpgplayer_character (delegate Custom|PlayerDead_Event_0)))

(fn ConstructionScript)